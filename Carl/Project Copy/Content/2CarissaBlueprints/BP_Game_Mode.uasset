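; Game mode Blueprint that respawns the first-person player character when it is destroyed.
; BeginPlay binds to the pawn's OnDestroyed event, which fades the camera out, waits, spawns a new character at SpawnTransform, possesses it and calls Respawn to rebind.
; A minutes/seconds countdown that would show a GameOver widget and pause the game is present but disconnected, so it never runs.
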(event `self.ReceiveBeginPlay`
  ;[1 1 1] Checkpoint Respawn BP
  (bind _asbp_player_pawn (cast `/Game/FirstPersonBP/Blueprints/FirstPersonCharacter` (`GameplayStatics.GetPlayerPawn` 0) :!label _label))
  (add `self.OnDestroyed` _asbp_player_pawn (delegate `OnDestroyed Event`)))

(event `Respawn`
  ;[1 1 1] Checkpoint Respawn BP
  (goto _label))

(event `OnDestroyed Event` :!signature `self.OnDestroyed`
  (params (DestroyedActor :type "Actor Object Reference"))
  ;[1 1 1] Checkpoint Respawn BP
  (`PlayerCameraManager.StartCameraFade` :`self` (`GameplayStatics.GetPlayerCameraManager` 0) :`ToAlpha` 1.0 :`Duration` 1.0)
  (`KismetSystemLibrary.Delay` 1.0)
  (bind _returnvalue (`|SpawnActorFromClass` "/Game/FirstPersonBP/Blueprints/FirstPersonCharacter.FirstPersonCharacter_C" (`self.Spawn Transform`) "AdjustIfPossibleButAlwaysSpawn" "OverrideRootScale" null null))
  (`Controller.Possess` (`GameplayStatics.GetPlayerController` 0) _returnvalue)
  (`self.Respawn`))

(event `self.ReceiveTick`
  (params (DeltaSeconds :type "Float (single-precision)"))
  ;[1 1 1] Timer BP
)

(fn `UserConstructionScript`)